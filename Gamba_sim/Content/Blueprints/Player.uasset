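; Player is a flipbook-animated character that the player moves along the world X and Y axes.
; MoveRight and MoveDown axis inputs feed movement input along positive X and Y respectively.
; Every tick, UpdateAnimation switches the sprite between the Tanaka walk and idle flipbooks based on whether the character has any velocity, with no directional variants.
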(event Custom|UpdateAnimation
  (Sprite|SetFlipbook (Variables|Default|GetSprite) (select (> (Math|Vector|VectorLength (Variables|/Script/Engine.MovementComponent|GetVelocity (Variables|Character|GetCharacterMovement))) 0.0) "/Game/Sprites/tanaka_walk_anim.tanaka_walk_anim" "/Game/Sprites/idle_anim.idle_anim")))

(event EventTick
  (params (DeltaSeconds :type Float%20%28single-precision%29))
  (CallFunction|UpdateAnimation))

(event Input|AxisEvents|InputAxisMoveRight
  (params (AxisValue :type Float%20%28single-precision%29))
  (Pawn|Input|AddMovementInput "1.000000,0.000000,0.000000" AxisValue false))

(event Input|AxisEvents|InputAxisMoveDown
  (params (AxisValue :type Float%20%28single-precision%29))
  (Pawn|Input|AddMovementInput "0.000000,1.000000,0.000000" AxisValue false))

(fn ConstructionScript)